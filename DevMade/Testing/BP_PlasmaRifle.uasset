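; BP_PlasmaRifle is a test Blueprint for an automatic rifle that spawns projectiles while firing.
; StartFiring starts a looping timer that calls FireProjectile every fifth of a second, and StopFiring clears it by handle.
; FireProjectile spawns an actor at the FiringBarrel component's world location, facing along its forward vector.
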(event Custom|StartFiring
  (bind _returnvalue (Utilities|Time|SetTimerbyFunctionName 0 "FireProjectile" 0.2 true))
  (bind _output_get (Variables|Default|SetFiringTimerHandle%20 _returnvalue)))

(event Custom|StopFiring
  (Utilities|Time|ClearandInvalidateTimerbyHandle (stale Custom|StartFiring _output_get)))

(fn ConstructionScript)

(fn FireProjectile
  (Game|SpawnActorfromClass "/Game/DevMade/Testing/BP_PlasmaProjectile.BP_PlasmaProjectile_C" (Math|Transform|MakeTransform (Transformation|GetWorldLocation (Variables|Default|GetFiringBarrel)) (Math|Rotator|MakeRotfromX (Math|Vector|GetForwardVector (Transformation|GetWorldRotation (Variables|Default|GetFiringBarrel))))) "Undefined" "MultiplyWithRoot" 0 0))